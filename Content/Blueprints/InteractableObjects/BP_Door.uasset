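; BP_Door is an interactable door that knocks when a BP_UseHitBox overlaps it, then "opens" to award the player candy.
; The overlap starts a looping timer that plays a 2D knock sound and counts down from KnockMax.
; When the count runs out, a delayed timer prints an opened message and adds one candy through the BP_Globals actor.
; The door itself never moves or changes visually in these graphs.
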(event EventBeginPlay)

(event Collision|EventActorBeginOverlap
  (params (OtherActor :type Actor%20Object%20Reference))
  (Utilities|Casting|CastToBP_UseHitBox OtherActor)
  (Development|PrintString "Door: You interacted with me :3")
  (CallFunction|PlayerOpenDoor))

(event EventTick
  (params (DeltaSeconds :type Float%20%28single-precision%29)))

(fn ConstructionScript)

(fn PlayerOpenDoor
  (Variables|Default|SetKnock_Counter (Variables|Default|GetKnock_Max))
  (Utilities|Time|SetTimerbyFunctionName 0 "Timer_Play_Knock" (Variables|Default|GetKnock_Delay) true))

(fn TimerPlayKnock
  (if (Math|Conversions|ToBoolean(Integer) (Variables|Default|GetKnock_Counter))
    ;[1 1 1] Decrement timer
    (Variables|Default|SetKnock_Counter (- (Variables|Default|GetKnock_Counter) 1))
    ;[1 1 1] Play knock sound
    (Audio|PlaySound2D "/Game/Assets/Sounds/Door/knock2.knock2" 1.0 1.0 0.0 0 0)
    (else
      ;[1 1 1] If we've knocked Knock_Max times, end timer
      (Utilities|Time|ClearTimerbyFunctionName 0 "Timer_Play_Knock")
      ;[1 1 1] DOOR STUCK! DOOR STUCK! PLEASE! I BEG YOU! WE'RE DEAD!
      (Utilities|Time|SetTimerbyFunctionName 0 "Timer_Door_Opening" (Variables|Default|GetDoor_Open_Delay)))))

(fn TimerDoorOpening
  (Development|PrintString "Door: Opened")
  (bind _returnvalue (Actor|GetActorOfClass "/Game/Blueprints/Global/BP_Globals.BP_Globals_C"))
  (Default|AddCandyAmount _returnvalue 1))