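; BP_Usable_Door_NoCandy is an interactable door that turns the player away with a rude speech bubble instead of opening.
; On BeginPlay it spawns a BP_Block at its own transform.
; PlayerUse starts a looping timer that plays a set number of knock sounds, then a delayed timer spawns the BP_SpeechBubble.
; The bubble uses a fixed offset, with a todo noting its Y axis depends on the tilemap.
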(event EventBeginPlay
  (|CallParentFunction)
  (CallFunction|SpawnBlock))

(event Collision|EventActorBeginOverlap
  (params (OtherActor :type Actor%20Object%20Reference))
  (|CallParentFunction OtherActor) ; This node is disabled and will not be called.\nDrag off pins to build functionality.
)

(event EventTick
  (params (DeltaSeconds :type Float%20%28single-precision%29))
  (|CallParentFunction DeltaSeconds) ; This node is disabled and will not be called.\nDrag off pins to build functionality.
)

(event EventPlayerUse
  (params (BP_Player :type BP%20Player%20Object%20Reference))
  (OnInteract|PlayerOpenDoor))

(fn ConstructionScript
  (|CallParentFunction))

(fn PlayerOpenDoor
  (Variables|Knocking|SetKnock_Counter (Variables|Knocking|GetKnock_Max))
  (Utilities|Time|SetTimerbyFunctionName 0 "Timer_Play_Knock" (Variables|Knocking|GetKnock_Delay) true))

(fn TimerPlayKnock
  (if (Math|Conversions|ToBoolean(Integer) (Variables|Knocking|GetKnock_Counter))
    ;[1 1 1] Decrement timer
    (Variables|Knocking|SetKnock_Counter (- (Variables|Knocking|GetKnock_Counter) 1))
    ;[1 1 1] Play knock sound
    (Audio|PlaySound2D "/Game/Assets/Sounds/Door/knock2.knock2" 1.0 1.0 0.0 0 0)
    (else
      ;[1 1 1] If we've knocked Knock_Max times, end timer
      (Utilities|Time|ClearTimerbyFunctionName 0 "Timer_Play_Knock")
      ;[1 1 1] DOOR STUCK! DOOR STUCK! PLEASE! I BEG YOU! WE'RE DEAD!
      (Utilities|Time|SetTimerbyFunctionName 0 "Timer_Door_Opening" (Variables|Knocking|GetDoor_Open_Delay)))))

(fn TimerDoorOpening
  (bind _returnvalue (Transformation|GetActorTransform))
  (bind _returnvalue_2 (Game|SpawnActorfromClass "/Game/Blueprints/SpeechBubble/BP_SpeechBubble.BP_SpeechBubble_C" _returnvalue "Undefined" 0 0))
  (Default|SetSpeechBubbleParam _returnvalue_2 "/Game/Assets/PNG/SpeechBubbles/S_SpeechBubble_Door_FuckOff.S_SpeechBubble_Door_FuckOff" 2.0 (+ (.Location (Math|Transform|BreakTransform _returnvalue)) "0,100.000000,40.000000")))

(fn SpawnBlock
  (Game|SpawnActorfromClass "/Game/Blueprints/AI/BP_Block.BP_Block_C" (Transformation|GetActorTransform) "AlwaysSpawn" 0 0))