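; BP_Globals is a global state actor that holds the game's candy and bone counters, clock and knock-attempt count.
; A looping timer started on BeginPlay advances a minute counter that wraps daily, with helpers returning 12-hour time and AM/PM.
; Adding candy also plays a random pickup sound.
; Reaching the knock target awards an achievement through WBP_Achievements widgets, and resets apply only while the count has not exceeded that target.
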(event EventBeginPlay
  (Utilities|Time|SetTimerbyFunctionName 0 "Timer_Minutes_Running" (Variables|Timer|GetTimer_Update_Rate) true))

(event Collision|EventActorBeginOverlap
  (params (OtherActor :type Actor%20Object%20Reference)))

(event EventTick
  (params (DeltaSeconds :type Float%20%28single-precision%29)))

(fn ConstructionScript)

(fn AddCandyAmount
  (params (Amount :type Integer))
  (Variables|CandyAndCurrency|SetCandyCounter (+ Amount (Variables|CandyAndCurrency|GetCandyCounter)))
  (CallFunction|PlayCandySound))

(fn AddBoneAmount
  (params (Amount :type Integer))
  (Variables|CandyAndCurrency|SetBoneCounter (+ Amount (Variables|CandyAndCurrency|GetBoneCounter))))

(fn TimeIsAM
  ;[1 1 1] 12:00 = 12 * 60 = 720
  (return (< (Variables|Timer|GetMinutesCounter) 720)))

(fn TimeGetHour
  (if (< (Variables|Timer|GetMinutesCounter) 60)
    (return 12)
    (elif (> (/ (Variables|Timer|GetMinutesCounter) 60) 12)
      (return (- (/ (Variables|Timer|GetMinutesCounter) 60) 12))
      (else
        (return (/ (Variables|Timer|GetMinutesCounter) 60))))))

(fn TimeGetMinute
  (return (Math|Integer|%(Integer) (Variables|Timer|GetMinutesCounter) 60)))

(fn TimerMinutesRunning
  (Variables|Timer|SetMinutesCounter (Math|Integer|%(Integer) (+ (Variables|Timer|GetMinutesCounter) (Variables|Timer|GetTimer_Update_Amt)) 1440)))

(fn PlayCandySound
  (switch int (Math|Random|RandomIntegerinRange 0 6)
    (:0
      (Audio|PlaySound2D "/Game/Assets/Sounds/Player/Pickup/Pickup1.Pickup1" 1.0 1.0 0.0 0 0))
    (:1
      (Audio|PlaySound2D "/Game/Assets/Sounds/Player/Pickup/Pickup2.Pickup2" 1.0 1.0 0.0 0 0))
    (:2
      (Audio|PlaySound2D "/Game/Assets/Sounds/Player/Pickup/Pickup3.Pickup3" 1.0 1.0 0.0 0 0))
    (:3
      (Audio|PlaySound2D "/Game/Assets/Sounds/Player/Pickup/Pickup4.Pickup4" 1.0 1.0 0.0 0 0))
    (:4
      (Audio|PlaySound2D "/Game/Assets/Sounds/Player/Pickup/Pickup5.Pickup5" 1.0 1.0 0.0 0 0))
    (:5
      (Audio|PlaySound2D "/Game/Assets/Sounds/Player/Pickup/Pickup6.Pickup6" 1.0 1.0 0.0 0 0))
    (:6
      (Audio|PlaySound2D "/Game/Assets/Sounds/Player/Pickup/Pickup7_best.Pickup7_best" 1.0 1.0 0.0 0 0))))

(fn IncrementKnockAttempts
  (bind _output_get (Variables|Default|SetTotalKnockAttempts (+ (Variables|Default|GetTotalKnockAttempts) 1)))
  (if (== _output_get (Variables|Default|GetTotalKnockAchievement))
    (bind _foundwidgets (Widget|GetAllWidgetsOfClass "/Game/Blueprints/HUD/WBP_Achievements.WBP_Achievements_C" true))
    (for _array_element _foundwidgets
      (Default|EarnAchievement _array_element 3))))

(fn ResetKnockAttempts
  (if (<= (Variables|Default|GetTotalKnockAttempts) (Variables|Default|GetTotalKnockAchievement))
    (Variables|Default|SetTotalKnockAttempts 0)))