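; Player character for a 2D sprite game, moving on the X/Z plane with Flying movement mode re-applied every Tick.
; Dash launches the character along its scaled velocity, with function-name timers ending it and its cooldown; a Todo notes it breaks movement.
; Tick swaps the sprite between normal, dash-ready and dashing states, and prints velocity and falling debug.
; Attack only runs a cooldown, while Interact and Inventory just print messages.
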(event EventBeginPlay
  (Development|PrintString "Player: Spawned"))

(event Collision|EventActorBeginOverlap
  (params (OtherActor :type Actor%20Object%20Reference)))

(event EventTick
  (params (DeltaSeconds :type Float%20%28single-precision%29))
  (CallFunction|AnimationStateMachine)
  (Development|PrintString (Utilities|String|ToString(Vector) (Transformation|GetVelocity)) true true "(R=0.000000,G=0.660000,B=1.000000,A=1.000000)" 0.0)
  (Development|PrintString (Utilities|String|ToString(Boolean) (AI|Components|NavMovement|IsFalling (Variables|Character|GetCharacterMovement))) true true "(R=1.000000,G=0.000000,B=0.299157,A=1.000000)" 0.0)
  (Pawn|Components|CharacterMovement|SetMovementMode (Variables|Character|GetCharacterMovement) "MOVE_Flying" 0))

(event Input|ActionEvents|InputActionInventory
  (params (Key :type Key%20Structure :default "None"))
  ;[1 1 1] Player Input
  (:Pressed
    (Development|PrintString "Player: Todo: Add inventory")))

(event Input|ActionEvents|InputActionDodge
  (params (Key :type Key%20Structure :default "None"))
  ;[1 1 1] Player Input
  (:Pressed
    (CallFunction|DoDash)))

(event Input|ActionEvents|InputActionInteract
  (params (Key :type Key%20Structure :default "None"))
  ;[1 1 1] Player Input
  (:Pressed
    (Development|PrintString "Player: Interacting")))

(event Input|ActionEvents|InputActionAttack
  (params (Key :type Key%20Structure :default "None"))
  ;[1 1 1] Player Input
  (:Pressed
    (CallFunction|DoAttack)))

(event Input|AxisEvents|InputAxisLeftOrRight
  (params (AxisValue :type Float%20%28single-precision%29))
  ;[1 1 1] Player Movement
  (Pawn|Input|AddMovementInput "1.000000, 0, 0" AxisValue false))

(event Input|AxisEvents|InputAxisUpOrDown
  (params (AxisValue :type Float%20%28single-precision%29))
  ;[1 1 1] Player Movement
  (Pawn|Input|AddMovementInput "0.000000, 0,1.000000" AxisValue false))

(fn ConstructionScript)

(fn AnimationStateMachine
  ;[1 1 1] Show Dash state
  (if (Variables|Default|GetIsDashing)
    (Rendering|Components|Sprite|SetSprite (Variables|Default|GetPaperSprite) "/Game/Assets/PNG/Test/S_Player_Dashing.S_Player_Dashing")
    (elif (Variables|Default|GetCanDash)
      (Rendering|Components|Sprite|SetSprite (Variables|Default|GetPaperSprite) "/Game/Assets/PNG/Test/S_Player_CanDash.S_Player_CanDash")
      (else
        (Rendering|Components|Sprite|SetSprite (Variables|Default|GetPaperSprite) "/Game/Assets/PNG/Test/S_Player.S_Player")))))

(fn TimerCanDashReset
  (Variables|Default|SetCanDash true)
  (Development|PrintString "Player: CanDash!"))

(fn TimerDashOver
  (Variables|Default|SetIsDashing false)
  (Development|PrintString "Player: Dash over"))

(fn DoDash
  (if (Variables|Default|GetCanDash)
    (Variables|Default|SetIsDashing true)
    (Variables|Default|SetCanDash false)
    (Utilities|Time|SetTimerbyFunctionName 0 "Timer_Dash_Over" (Variables|Default|GetDashTime))
    (Utilities|Time|SetTimerbyFunctionName 0 "Timer_Can_Dash_Reset" (Variables|Default|GetDash_Cooldown))
    ;[1 1 1] Todo: This breaks player movement... Fix this!
    (Character|LaunchCharacter (* (Transformation|GetVelocity) (Variables|Default|GetDash_Multiplier)) false false)
    (Development|PrintString "Player: Dashing!")
    (else
      (Development|PrintString "Player: Cannot Dash ATM"))))

(fn DoAttack
  (if (Variables|Default|GetCanAttack)
    (Variables|Default|SetCanAttack false)
    (Utilities|Time|SetTimerbyFunctionName 0 "Timer_Can_Attack_Reset" (Variables|Default|GetAttack_Cooldown))
    (Development|PrintString "Player: Attacking!")
    (else
      (Development|PrintString "Player: Cannot attack yet"))))

(fn TimerCanAttackReset
  (Variables|Default|SetCanAttack true)
  (Development|PrintString "Player: Attack cooldown over!"))