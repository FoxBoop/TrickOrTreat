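; An easter egg pickup point that awards an achievement when the player gets close to it.
; On BeginPlay it picks its paper sprite from EasterEggID and starts a looping timer.
; The timer polls the distance to BP_Player instead of using overlap events or Tick.
; While the player is within the small fixed radius, it calls EarnAchievement with the ID on every top-level WBP_Achievements widget.
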(event EventBeginPlay
  (bind _papersprite (Variables|Default|GetPaperSprite))
  (Utilities|Time|SetTimerbyFunctionName 0 "Timer_Think" 0.2 true)
  (switch int (Variables|Default|GetEasterEggID)
    (:0
      (Rendering|Components|Sprite|SetSprite _papersprite "/Game/Assets/PNG/Bingus/S_Bingus.S_Bingus"))
    (:1
      (Rendering|Components|Sprite|SetSprite _papersprite "/Game/Assets/PNG/Bone/S_Bone.S_Bone"))))

(event Collision|EventActorBeginOverlap
  (params (OtherActor :type Actor%20Object%20Reference)))

(event EventTick
  (params (DeltaSeconds :type Float%20%28single-precision%29)))

(fn ConstructionScript)

(fn WithinRadius
  (bind _returnvalue (Actor|GetActorOfClass "/Game/Blueprints/Player/BP_Player.BP_Player_C"))
  (if (Utilities|IsValid _returnvalue)
    (return (< (Math|Vector|Distance(Vector) (Transformation|GetActorLocation _returnvalue) (Transformation|GetActorLocation)) 75.0))))

(fn TimerThink
  (bind _inradius (CallFunction|WithinRadius))
  (if _inradius
    (bind _foundwidgets (Widget|GetAllWidgetsOfClass "/Game/Blueprints/HUD/WBP_Achievements.WBP_Achievements_C" true))
    (for _array_element _foundwidgets
      (Default|EarnAchievement _array_element (Variables|Default|GetEasterEggID)))))