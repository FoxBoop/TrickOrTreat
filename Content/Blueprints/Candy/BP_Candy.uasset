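; BP_Candy is a candy pickup that shows one of seven random Paper2D sprites, chosen on BeginPlay.
; Each tick, once the player is within range, it eases toward them by a swept fraction of the gap, with MoveSpeed as a frame-rate-dependent divisor.
; Overlapping BP_Player destroys it and adds random points to BP_Globals' candy count.
; PlayPickupSound is called but empty, as its random-sound logic is disconnected.
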(event OnComponentBeginOverlap(Box)
  (params (OverlappedComponent :type Primitive%20Component%20Object%20Reference) (OtherActor :type Actor%20Object%20Reference) (OtherComp :type Primitive%20Component%20Object%20Reference) (OtherBodyIndex :type Integer) (bFromSweep :type Boolean) (SweepResult :type Hit%20Result%20Structure%20%28by%20ref%29))
  ;[1 1 1] On touching the player
  (Utilities|Casting|CastToBP_Player OtherActor)
  (CallFunction|PlayPickupSound)
  (Actor|DestroyActor)
  (bind _returnvalue (Actor|GetActorOfClass "/Game/Blueprints/Global/BP_Globals.BP_Globals_C"))
  (Default|AddCandyAmount _returnvalue (Math|Random|RandomIntegerinRange (Variables|Default|GetCandy_Points_Min) (Variables|Default|GetCandy_Points_Max))))

(event EventBeginPlay
  (CallFunction|SetRandomCandySprite))

(event Collision|EventActorBeginOverlap
  (params (OtherActor :type Actor%20Object%20Reference)))

(event EventTick
  (params (DeltaSeconds :type Float%20%28single-precision%29))
  (CallFunction|MovetoPlayer))

(fn ConstructionScript)

(fn SetRandomCandySprite
  (bind _papersprite (Variables|Default|GetPaperSprite))
  ;[1 1 1] These branches... wow
  (switch int (Math|Random|RandomInteger 7)
    (:0
      (Rendering|Components|Sprite|SetSprite _papersprite "/Game/Assets/PNG/Candy/S_Candy_1.S_Candy_1"))
    (:1
      (Rendering|Components|Sprite|SetSprite _papersprite "/Game/Assets/PNG/Candy/S_Candy_2.S_Candy_2"))
    (:2
      (Rendering|Components|Sprite|SetSprite _papersprite "/Game/Assets/PNG/Candy/S_Candy_3.S_Candy_3"))
    (:3
      (Rendering|Components|Sprite|SetSprite _papersprite "/Game/Assets/PNG/Candy/S_Candy_4.S_Candy_4"))
    (:4
      (Rendering|Components|Sprite|SetSprite _papersprite "/Game/Assets/PNG/Candy/S_Candy_5.S_Candy_5"))
    (:5
      (Rendering|Components|Sprite|SetSprite _papersprite "/Game/Assets/PNG/Candy/S_Candy_6.S_Candy_6"))
    (:6
      (Rendering|Components|Sprite|SetSprite _papersprite "/Game/Assets/PNG/Candy/S_Candy_7.S_Candy_7"))))

(fn MovetoPlayer
  (if (< (Math|Vector|Distance(Vector) (Transformation|GetActorLocation) (Transformation|GetActorLocation (Game|Player|GetPlayerPawn 0))) (Variables|Default|GetPlayer_Distance_Move))
    ;[1 1 1] Move to player
    (Transformation|SetActorLocation (+ (Transformation|GetActorLocation) (/ (- (Transformation|GetActorLocation (Game|Player|GetPlayerPawn 0)) (Transformation|GetActorLocation)) (Variables|Default|GetMove_Speed))) true false)))

(fn PlayPickupSound)