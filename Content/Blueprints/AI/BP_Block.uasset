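; BP_Block is a placed zone that awards an achievement when the player stays inside it long enough while monsters camp nearby.
; A looping timer checks whether the player is within the scaled sphere's radius and any Skeliboi or Skinwalker is within twice that radius, using distance tests instead of overlaps.
; Time accumulates while both hold and resets otherwise; reaching the threshold awards the achievement through BP_GameInstance.
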(event EventBeginPlay
  (Transformation|SetRelativeScale3D (Variables|Default|GetSphere) "2.500000,2.500000,2.500000")
  (Utilities|Time|SetTimerbyFunctionName 0 "timer_check" (Variables|Default|Gettimer_loop_time) true))

(event Collision|EventActorBeginOverlap
  (params (OtherActor :type Actor%20Object%20Reference)))

(event EventTick
  (params (DeltaSeconds :type Float%20%28single-precision%29)))

(fn ConstructionScript)

(fn TimerCheck
  ;[1 1 1] Is player in radius and monsters are camping near by?
  (bind _returnvalue (Actor|GetActorOfClass "/Game/Blueprints/Player/BP_Player.BP_Player_C"))
  (bind _is_close_and_outside (CallFunction|IsVectorinSphere (Transformation|GetActorLocation _returnvalue)))
  (if _is_close_and_outside
    (bind _monster_is_near_by (CallFunction|IsMonsterClose))
    (if _monster_is_near_by
      ;;[1 1 1] Increment timer....
      (Variables|Default|Settime_player_close (+ (Variables|Default|Gettime_player_close) (Variables|Default|Gettimer_loop_time)))
      ;[1 1 1] Earn achievement
      (CallFunction|CallAchievement)
      (else
        (Variables|Default|Settime_player_close 0.0)))
    (else
      (Variables|Default|Settime_player_close 0.0))))

(fn IsVectorinSphere
  (params (vector :type Vector))
  (return (<= (Math|Vector|Distance(Vector) vector (Transformation|GetActorLocation)) (Components|Sphere|GetScaledSphereRadius (Variables|Default|GetSphere)))))

(fn IsVectorClose
  (params (vec :type Vector))
  (return (<= (Math|Vector|Distance(Vector) vec (Transformation|GetActorLocation)) (* (Components|Sphere|GetScaledSphereRadius (Variables|Default|GetSphere)) 2.0))))

(fn IsMonsterClose
  ;[1 1 1] Are skeliboys close?
  (bind _outactors (Actor|GetAllActorsOfClass "/Game/Blueprints/AI/Skeliboi/BP_Skeliboi.BP_Skeliboi_C"))
  (for _array_element _outactors
    (bind _within_radius (CallFunction|IsVectorClose (Transformation|GetActorLocation _array_element)))
    (if _within_radius
      (return true)))
  ;[1 1 1] Are skin... things... close?
  (bind _outactors_2 (Actor|GetAllActorsOfClass "/Game/Blueprints/AI/Skinwalker/BP_Skinwalker.BP_Skinwalker_C"))
  (for _array_element_2 _outactors_2
    (bind _within_radius_2 (CallFunction|IsVectorClose (Transformation|GetActorLocation _array_element_2)))
    (if _within_radius_2
      (return true))))

(fn CallAchievement
  (if (>= (Variables|Default|Gettime_player_close) (Variables|Default|Gettime_achievement))
    (bind _asbp_game_instance (Utilities|Casting|CastToBP_GameInstance (Game|GetGameInstance)))
    (Default|AchievementEarn _asbp_game_instance 11)))