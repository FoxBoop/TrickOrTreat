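; BP_Child_Spawner is an AI spawner that randomly creates BP_Child_Test pawns while its location is off screen.
; A looping timer started on BeginPlay runs Timer_Think, which rolls against ChanceOfSpawning whenever On_Screen returns false.
; On_Screen projects the spawner's location through player controller 0 and compares it with the viewport bounds, ignoring the projection's success result.
; Create_Child spawns the AI at the spawner's location and rotation and prints a debug message.
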(event EventBeginPlay
  (Utilities|Time|SetTimerbyFunctionName 0 "Timer_Think" (Variables|Default|GetSpawn_Timer_Time) true))

(event Collision|EventActorBeginOverlap
  (params (OtherActor :type Actor%20Object%20Reference)))

(event EventTick
  (params (DeltaSeconds :type Float%20%28single-precision%29)))

(fn ConstructionScript)

(fn DoSpawn
  ;[1 1 1] Chance of spawning
  (return (< (Math|Random|RandomFloat) (Variables|Default|GetChanceOfSpawning))))

(fn TimerThink
  ;[1 1 1] If spawner is not on screen, then possibly spawn child
  (bind _onscreen (CallFunction|OnScreen))
  (if (not _onscreen)
    ;[1 1 1] Spawn child
    (bind _dospawn (CallFunction|DoSpawn))
    (if _dospawn
      (CallFunction|CreateChild))))

(fn OnScreen
  (bind _returnvalue (Viewport|GetViewportSize))
  (bind _returnvalue_2 (Game|GetPlayerController 0))
  (bind _returnvalue_3 (Transformation|GetActorLocation))
  (bind (_x _y) (Math|Vector2D|BreakVector2D _returnvalue))
  (bind _screenposition (Class|GameplayStatics|ProjectWorldtoScreen _returnvalue_2 _returnvalue_3 false))
  (bind (_x_2 _y_2) (Math|Vector2D|BreakVector2D _screenposition))
  (return (not (Math|Boolean|ORBoolean (> _x_2 _x) (> _y_2 _y) (< _x_2 0.0) (< _y_2 0.0)))))

(fn CreateChild
  (bind _returnvalue (Transformation|GetActorTransform))
  (bind (_location _rotation) (Math|Transform|BreakTransform _returnvalue))
  (AI|SpawnAIFromClass "/Game/Blueprints/AI/BP_Child_Test.BP_Child_Test_C" 0 _location _rotation false 0)
  (Development|PrintString "Spawned actor"))