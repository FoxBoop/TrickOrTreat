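; A Paper2D child pawn that is a disguised skinwalker, walking sideways and replacing itself with BP_Skinwalker when the player comes within range.
; Tick flips the flipbook by velocity, moves along a random or forced X direction, and runs the proximity check; the old candy-spawning code is disconnected.
; If no direction is preset at BeginPlay, timers destroy it after it leaves the screen, or after a timeout if never seen.
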(event EventBeginPlay
  ;[1 1 1] Only a random direction if none is set
  (if (== (.X (Math|Vector|BreakVector (Variables|Default|GetMove_Direction))) 0.0)
    ;[1 1 1] Create movement direction
    (bind _dir (CallFunction|RandomDir))
    (Variables|Default|SetMove_Direction (Math|Vector|MakeVector (Math|Conversions|ToFloat(Integer) _dir) 0.0 0.0))
    ;[1 1 1] If actor doesn't get deleted within 30 seconds, force delete
    (Utilities|Time|SetTimerbyFunctionName 0 "Timer_Force_Delete" 3e+01)
    ;[1 1 1] Do normal delete logic
    (Utilities|Time|SetTimerbyFunctionName 0 "Timer_Think" 0.1 true)))

(event Collision|EventActorBeginOverlap
  (params (OtherActor :type Actor%20Object%20Reference)))

(event EventTick
  (params (DeltaSeconds :type Float%20%28single-precision%29))
  ;[1 1 1] Walk and rotate
  (CallFunction|Rotation)
  (Pawn|Input|AddMovementInput (Variables|Default|GetMove_Direction) (Variables|Default|GetMovementSpeed) false)
  ;[1 1 1] Check if we should spawn candy
  (bind _dodrop (CallFunction|DoDropCandy))
  (if _dodrop
    (CallFunction|DropCandy)))

(fn ConstructionScript)

(fn TimerThink
  ;[1 1 1] On screen, mark for delete
  (bind _onscreen (CallFunction|OnScreen))
  (if _onscreen
    (Variables|Default|SetMarkForDelete true)
    (else
      ;[1 1 1] Not on screen and marked for delete... delet dis!
      (if (and (not _onscreen) (Variables|Default|GetMarkForDelete))
        (Actor|DestroyActor)
        (Development|PrintString "Out of view, deleted")))))

(fn RandomDir
  (if (Math|Random|RandomBool)
    (return 1)
    (else
      (return -1))))

(fn TimerForceDelete
  ;[1 1 1] Actor was not ever on screen, and timer ran out... Delete actor
  (if (not (Variables|Default|GetMarkForDelete))
    (Actor|DestroyActor)))

(fn OnScreen
  (bind _returnvalue (Viewport|GetViewportSize))
  (bind _returnvalue_2 (Game|GetPlayerController 0))
  (bind _returnvalue_3 (Transformation|GetActorLocation))
  (bind (_x _y) (Math|Vector2D|BreakVector2D _returnvalue))
  (bind _screenposition (Class|GameplayStatics|ProjectWorldtoScreen _returnvalue_2 _returnvalue_3 false))
  (bind (_x_2 _y_2) (Math|Vector2D|BreakVector2D _screenposition))
  (return (not (Math|Boolean|ORBoolean (> _x_2 _x) (> _y_2 _y) (< _x_2 0.0) (< _y_2 0.0)))))

(fn DoDropCandy
  (bind _returnvalue (Game|Player|GetPlayerPawn 0))
  (if (Utilities|IsValid _returnvalue)
    (return (and (< (Math|Vector|Distance(Vector) (Transformation|GetActorLocation) (Transformation|GetActorLocation _returnvalue)) (Variables|Default|GetDrop_Candy_Distance)) (not (Variables|Default|GetDroppedCandy))))))

(fn DropCandy
  (bind _returnvalue (Transformation|GetActorTransform))
  (bind (_location _rotation) (Math|Transform|BreakTransform _returnvalue))
  ;[1 1 1] Don't drop candy more than once
  (Variables|Default|SetDroppedCandy true)
  ;[1 1 1] Remove "disguise"!
  (AI|SpawnAIFromClass "/Game/Blueprints/AI/Skinwalker/BP_Skinwalker.BP_Skinwalker_C" 0 _location _rotation false 0)
  (Actor|DestroyActor))

(fn Rotation
  ;[1 1 1] If player is moving to the right, set flipbook rotation
  (if (> (.X (Math|Vector|BreakVector (Transformation|GetVelocity))) 0.0)
    (Transformation|SetRelativeRotation (Variables|Default|GetPaperFlipbook) "0, 0, 0" false false)
    (else
      ;[1 1 1] Check if player is moving to the left, set flipbook rotation
      (if (< (.X (Math|Vector|BreakVector (Transformation|GetVelocity))) 0.0)
        (Transformation|SetRelativeRotation (Variables|Default|GetPaperFlipbook) "0,180.000000,0.000000" false false)))))

(fn ForceDirection
  (params (float_new_x :type Float%20%28single-precision%29))
  (if (!= float_new_x 0.0)
    (Variables|Default|SetMove_Direction (Math|Vector|MakeVector float_new_x 0.0 0.0))))