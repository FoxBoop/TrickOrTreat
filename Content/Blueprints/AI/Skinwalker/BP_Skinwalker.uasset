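; BP_Skinwalker is a flipbook-animated enemy that chases the player, attacks in melee and dies ten seconds after spawning.
; Tick flips the sprite by X velocity, then either walks toward the player or attacks when within reach.
; Name-based timers sized from flipbook length apply damage near mid-swing after re-checking range, reset the attack, and destroy the actor after its death animation.
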(event EventBeginPlay
  ;[1 1 1] Despawn in 10 seconds
  (Utilities|Time|SetTimerbyFunctionName 0 "Timer_Die" 1e+01))

(event Collision|EventActorBeginOverlap
  (params (OtherActor :type Actor%20Object%20Reference)))

(event EventTick
  (params (DeltaSeconds :type Float%20%28single-precision%29))
  ;[1 1 1] AI logic, walking and attacking
  (CallFunction|AnimationRotationMachine)
  (bind _can_attack (CallFunction|IsWithinReach))
  (if _can_attack
    (CallFunction|StartAttack)
    (else
      (CallFunction|WalktoPlayer))))

(fn ConstructionScript)

(fn WalktoPlayer
  (bind _returnvalue (Game|Player|GetPlayerPawn 0))
  (if (not (or (Variables|Default|GetIsAttacking) (Variables|Default|GetIsDead)))
    (if (Utilities|IsValid _returnvalue)
      (Pawn|Input|AddMovementInput (- (Transformation|GetActorLocation _returnvalue) (Transformation|GetActorLocation)) 1.0 false))))

(fn IsWithinReach
  (bind _returnvalue (Actor|GetActorOfClass "/Game/Blueprints/Player/BP_Player.BP_Player_C"))
  (if (Utilities|IsValid _returnvalue)
    (return (< (Math|Vector|Distance(Vector) (Transformation|GetActorLocation _returnvalue) (Transformation|GetActorLocation)) (Variables|Default|GetAttackDistance)))))

(fn TimerDie
  (Sprite|SetFlipbook (Variables|Default|GetFB_Skinwalker_Walk) "/Game/Assets/PNG/AI/Skinwalker/Die/FB_Skinwalker_Die.FB_Skinwalker_Die")
  (Utilities|Time|SetTimerbyFunctionName 0 "Timer_Delete_Self" (Class|PaperFlipbookComponent|GetFlipbookLength (Variables|Default|GetFB_Skinwalker_Walk)))
  (Variables|Default|SetIsDead true))

(fn StartAttack
  (bind _fb_skinwalker_walk (Variables|Default|GetFB_Skinwalker_Walk))
  (bind _returnvalue (Class|PaperFlipbookComponent|GetFlipbookLength _fb_skinwalker_walk))
  (if (not (Variables|Default|GetIsAttacking))
    (Variables|Default|SetIsAttacking true)
    (Sprite|SetFlipbook (Variables|Default|GetFB_Skinwalker_Walk) "/Game/Assets/PNG/AI/Skinwalker/Attack/FB_Skinwalker_attack.FB_Skinwalker_attack")
    (Utilities|Time|SetTimerbyFunctionName 0 "Timer_Attack_Reset" _returnvalue)
    (Utilities|Time|SetTimerbyFunctionName 0 "Do_Player_Damage" (/ _returnvalue 2.1))))

(fn TimerAttackReset
  (Variables|Default|SetIsAttacking false)
  (Sprite|SetFlipbook (Variables|Default|GetFB_Skinwalker_Walk) "/Game/Assets/PNG/AI/Skinwalker/Walk/FB_Skinwalker_Walk.FB_Skinwalker_Walk"))

(fn TimerDeleteSelf
  (Actor|DestroyActor))

(fn DoPlayerDamage
  (bind _can_attack (CallFunction|IsWithinReach))
  (if _can_attack
    (bind _returnvalue (Actor|GetActorOfClass "/Game/Blueprints/Player/BP_Player.BP_Player_C"))
    (if (Utilities|IsValid _returnvalue)
      (Default|TakeDamage _returnvalue 15))))

(fn AnimationRotationMachine
  ;[1 1 1] If player is moving to the right, set flipbook rotation
  (if (> (.X (Math|Vector|BreakVector (Transformation|GetVelocity))) 0.0)
    (Transformation|SetRelativeRotation (Variables|Default|GetFB_Skinwalker_Walk) "0, 0, 0" false false)
    (else
      ;[1 1 1] Check if player is moving to the left, set flipbook rotation
      (if (< (.X (Math|Vector|BreakVector (Transformation|GetVelocity))) 0.0)
        (Transformation|SetRelativeRotation (Variables|Default|GetFB_Skinwalker_Walk) "0,180.000000,0.000000" false false)))))