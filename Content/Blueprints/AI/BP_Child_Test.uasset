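; Test child AI pawn that walks in a random direction along the X axis and drops candy once when the player comes within range.
; Tick drives movement and the distance check, spawning a random number of BP_Candy actors.
; A looping timer projects its location to screen space, destroying it once it leaves view after being seen.
; A 30-second fallback timer deletes children never seen on screen.
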(event EventBeginPlay
  ;[1 1 1] Create movement direction
  (bind _dir (CallFunction|RandomDir))
  (Variables|Default|SetMove_Direction (Math|Vector|MakeVector (Math|Conversions|ToFloat(Integer) _dir) 0.0 0.0))
  ;[1 1 1] If actor doesn't get deleted within 30 seconds, force delete
  (Utilities|Time|SetTimerbyFunctionName 0 "Timer_Force_Delete" 3e+01)
  ;[1 1 1] Do normal delete logic
  (Utilities|Time|SetTimerbyFunctionName 0 "Timer_Think" 0.1 true))

(event Collision|EventActorBeginOverlap
  (params (OtherActor :type Actor%20Object%20Reference)))

(event EventTick
  (params (DeltaSeconds :type Float%20%28single-precision%29))
  ;[1 1 1] Child will walk
  (Pawn|Input|AddMovementInput (Variables|Default|GetMove_Direction) (Variables|Default|GetMovementSpeed) false)
  ;[1 1 1] Check if we should spawn candy
  (bind _dodrop (CallFunction|DoDropCandy))
  (if _dodrop
    (CallFunction|DropCandy)))

(fn ConstructionScript)

(fn TimerThink
  ;[1 1 1] On screen, mark for delete
  (bind _onscreen (CallFunction|OnScreen))
  (if _onscreen
    (Variables|Default|SetMarkForDelete true)
    (else
      ;[1 1 1] Not on screen and marked for delete... delet dis!
      (if (and (not _onscreen) (Variables|Default|GetMarkForDelete))
        (Actor|DestroyActor)
        (Development|PrintString "Out of view, deleted")))))

(fn RandomDir
  (if (Math|Random|RandomBool)
    (return 1)
    (else
      (return -1))))

(fn TimerForceDelete
  ;[1 1 1] Actor was not ever on screen, and timer ran out... Delete actor
  (if (not (Variables|Default|GetMarkForDelete))
    (Actor|DestroyActor)
    (Development|PrintString "Force deleted actor")))

(fn OnScreen
  (bind _returnvalue (Viewport|GetViewportSize))
  (bind _returnvalue_2 (Game|GetPlayerController 0))
  (bind _returnvalue_3 (Transformation|GetActorLocation))
  (bind (_x _y) (Math|Vector2D|BreakVector2D _returnvalue))
  (bind _screenposition (Class|GameplayStatics|ProjectWorldtoScreen _returnvalue_2 _returnvalue_3 false))
  (bind (_x_2 _y_2) (Math|Vector2D|BreakVector2D _screenposition))
  (return (not (Math|Boolean|ORBoolean (> _x_2 _x) (> _y_2 _y) (< _x_2 0.0) (< _y_2 0.0)))))

(fn DoDropCandy
  (return (and (< (Math|Vector|Distance(Vector) (Transformation|GetActorLocation) (Transformation|GetActorLocation (Game|Player|GetPlayerPawn 0))) (Variables|Default|GetDrop_Candy_Distance)) (not (Variables|Default|GetDroppedCandy)))))

(fn DropCandy
  ;[1 1 1] Don't drop candy more than once
  (Variables|Default|SetDroppedCandy true)
  ;[1 1 1] Spawn N random candy actors
  (for _index (range (Math|Random|RandomIntegerinRange 0 (Variables|Default|GetCandy_Drop_Amount)) (Variables|Default|GetCandy_Drop_Amount))
    (Game|SpawnActorfromClass "/Game/Blueprints/Candy/BP_Candy.BP_Candy_C" (Transformation|GetActorTransform) "AdjustIfPossibleButAlwaysSpawn" 0 0)))