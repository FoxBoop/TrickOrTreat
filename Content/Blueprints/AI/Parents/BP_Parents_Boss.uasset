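; BP_Parents_Boss is a boss parent Blueprint with basic AI that chases the first player's pawn.
; Each Tick runs AIThink, which calls WalkToPlayer while AllowWalking is set, then forces the movement mode to Flying.
; WalkToPlayer feeds the unnormalized vector to the player into AddMovementInput, using direct steering without pathfinding, or a zero vector when no pawn is valid.
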(event EventBeginPlay)

(event Collision|EventActorBeginOverlap
  (params (OtherActor :type Actor%20Object%20Reference)))

(event EventTick
  (params (DeltaSeconds :type Float%20%28single-precision%29))
  (CallFunction|AIThink)
  (Pawn|Components|CharacterMovement|SetMovementMode (Variables|Character|GetCharacterMovement) "MOVE_Flying" 0))

(fn ConstructionScript)

(fn AIThink
  (if (Variables|Default|GetAllowWalking)
    (CallFunction|WalktoPlayer)))

(fn WalktoPlayer
  (bind _vector (CallFunction|VectortoPlayer))
  (Pawn|Input|AddMovementInput _vector 1.0 false))

(fn VectortoPlayer
  (bind _returnvalue (Game|Player|GetPlayerPawn 0))
  (if (Utilities|IsValid _returnvalue)
    (return (- (Transformation|GetActorLocation _returnvalue) (Transformation|GetActorLocation)))
    (else
      (return "0, 0, 0"))))