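; AI spawner that periodically spawns child, Skeliboi or Skinwalker child pawns while its location is outside the player's view.
; A looping timer projects the spawner's location to screen space and, when outside the viewport bounds, rolls against a spawn chance.
; Sequential percentage rolls pick Skeliboi, then Skinwalker, else a regular child, with odds scaled by the game instance's difficulty.
; Both child types receive the spawner's forced direction after spawning.
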(event EventBeginPlay
  (Utilities|Time|SetTimerbyFunctionName 0 "Timer_Think" (Variables|Default|GetSpawn_Timer_Time) true))

(event Collision|EventActorBeginOverlap
  (params (OtherActor :type Actor%20Object%20Reference)))

(event EventTick
  (params (DeltaSeconds :type Float%20%28single-precision%29)))

(fn ConstructionScript)

(fn DoSpawn
  ;[1 1 1] Chance of spawning
  (return (< (Math|Random|RandomFloat) (Variables|Default|GetChanceOfSpawning))))

(fn TimerThink
  ;[1 1 1] If spawner is not on screen, then possibly spawn child
  (bind _onscreen (CallFunction|OnScreen))
  (if (not _onscreen)
    ;[1 1 1] Spawn child
    (bind _dospawn (CallFunction|DoSpawn))
    (if _dospawn
      (CallFunction|CreateChild))))

(fn OnScreen
  (bind _returnvalue (Viewport|GetViewportSize))
  (bind _returnvalue_2 (Game|GetPlayerController 0))
  (bind _returnvalue_3 (Transformation|GetActorLocation))
  (bind (_x _y) (Math|Vector2D|BreakVector2D _returnvalue))
  (bind _screenposition (Class|GameplayStatics|ProjectWorldtoScreen _returnvalue_2 _returnvalue_3 false))
  (bind (_x_2 _y_2) (Math|Vector2D|BreakVector2D _screenposition))
  (return (not (Math|Boolean|ORBoolean (> _x_2 _x) (> _y_2 _y) (< _x_2 0.0) (< _y_2 0.0)))))

(fn CreateChild
  (bind _returnvalue (Transformation|GetActorTransform))
  (bind (_location _rotation) (Math|Transform|BreakTransform _returnvalue))
  (bind _ai_num (CallFunction|RandomEntity))
  (switch int _ai_num
    (:Default
      (bind _returnvalue_2 (AI|SpawnAIFromClass "/Game/Blueprints/AI/BP_Child_Test.BP_Child_Test_C" 0 _location _rotation false 0 :!label _label))
      (bind _asbp_child_test (Utilities|Casting|CastToBP_Child_Test _returnvalue_2))
      (Default|ForceDirection _asbp_child_test (Variables|Default|GetEditForceDirection)))
    (:0
      (goto _label))
    (:1
      (bind _returnvalue_3 (AI|SpawnAIFromClass "/Game/Blueprints/AI/Skeliboi/BP_Skeliboi.BP_Skeliboi_C" 0 _location _rotation false 0))
      (Utilities|Casting|CastToBP_Skeliboi _returnvalue_3))
    (:2
      (bind _returnvalue_4 (AI|SpawnAIFromClass "/Game/Blueprints/AI/Skinwalker/BP_Skinwalker_Child.BP_Skinwalker_Child_C" 0 _location _rotation false 0))
      (bind _asbp_skinwalker_child (Utilities|Casting|CastToBP_Skinwalker_Child _returnvalue_4))
      (Default|ForceDirection _asbp_skinwalker_child (Variables|Default|GetEditForceDirection)))))

(fn RandomEntity
  ;[1 1 1] chance of spawning skeliboi
  (bind _chance (CallFunction|SpawnChanceSkeliboi))
  (if (< (Math|Random|RandomIntegerinRange 0 99) _chance)
    (return 1)
    (else
      ;[1 1 1] Chance of spawning a NPCKid or Skinwalker
      (bind _chance_2 (CallFunction|SpawnChanceSkinwalker))
      (if (< (Math|Random|RandomIntegerinRange 0 99) _chance_2)
        (return 2)
        (else
          (return 0))))))

(fn SpawnChanceSkeliboi
  (bind _asbp_game_instance (Utilities|Casting|CastToBP_GameInstance (Game|GetGameInstance)))
  (switch int (Variables|/Game/Blueprints/GameInstance/BP_GameInstance.BP_GameInstance_C|GetDifficulty _asbp_game_instance)
    (:0
      ;[1 1 1] Easy
      (return 10))
    (:1
      ;[1 1 1] Normal
      (return 20))
    (:2
      ;[1 1 1] Hard
      (return 30))
    (:3
      ;[1 1 1] Inhuman
      (return 40))))

(fn SpawnChanceSkinwalker
  (bind _asbp_game_instance (Utilities|Casting|CastToBP_GameInstance (Game|GetGameInstance)))
  (switch int (Variables|/Game/Blueprints/GameInstance/BP_GameInstance.BP_GameInstance_C|GetDifficulty _asbp_game_instance)
    (:0
      ;[1 1 1] Easy
      (return 10))
    (:1
      ;[1 1 1] Normal
      (return 20))
    (:2
      ;[1 1 1] Hard
      (return 35))
    (:3
      ;[1 1 1] Inhuman
      (return 50))))