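; Skeliboi is a short-lived flipbook skeleton enemy, reusing Skinwalker AI, that chases the player and attacks in melee.
; Each Tick flips the sprite by X velocity, then either moves toward the player or attacks when within range.
; Flipbook-length timers drive attack reset and a mid-swing, range-rechecked hit scaled by GameInstance difficulty.
; A timer from BeginPlay plays its death animation after fifteen seconds, then destroys it.
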(event EventBeginPlay
  ;[1 1 1] Despawn in 15 seconds
  (Utilities|Time|SetTimerbyFunctionName 0 "Timer_Die" 15.0))

(event Collision|EventActorBeginOverlap
  (params (OtherActor :type Actor%20Object%20Reference)))

(event EventTick
  (params (DeltaSeconds :type Float%20%28single-precision%29))
  ;[1 1 1] Ai logic from Skinwalker
  (CallFunction|AnimationRotationMachine)
  (bind _can_attack (CallFunction|IsPlayerWithinRange))
  (if _can_attack
    (CallFunction|StartAttack)
    (else
      (CallFunction|WalktoPlayer))))

(fn ConstructionScript)

(fn WalktoPlayer
  (bind _returnvalue (Game|Player|GetPlayerPawn 0))
  (if (not (or (Variables|Default|GetIsAttacking) (Variables|Default|GetIsDead)))
    (if (Utilities|IsValid _returnvalue)
      (Pawn|Input|AddMovementInput (- (Transformation|GetActorLocation _returnvalue) (Transformation|GetActorLocation)) 1.0 false))))

(fn IsPlayerWithinRange
  (bind _returnvalue (Actor|GetActorOfClass "/Game/Blueprints/Player/BP_Player.BP_Player_C"))
  (if (Utilities|IsValid _returnvalue)
    (return (< (Math|Vector|Distance(Vector) (Transformation|GetActorLocation _returnvalue) (Transformation|GetActorLocation)) (Variables|Default|GetAttackDistance)))))

(fn TimerDie
  (Sprite|SetFlipbook (Variables|Default|GetFB_Skinwalker_Walk) "/Game/Assets/PNG/AI/Skeliboi/Die/FB_Skeliboi_Die.FB_Skeliboi_Die")
  (Utilities|Time|SetTimerbyFunctionName 0 "Timer_Delete_Self" (Class|PaperFlipbookComponent|GetFlipbookLength (Variables|Default|GetFB_Skinwalker_Walk)))
  (Variables|Default|SetIsDead true))

(fn StartAttack
  (bind _fb_skinwalker_walk (Variables|Default|GetFB_Skinwalker_Walk))
  (bind _returnvalue (Class|PaperFlipbookComponent|GetFlipbookLength _fb_skinwalker_walk))
  (if (not (Variables|Default|GetIsAttacking))
    (Variables|Default|SetIsAttacking true)
    (Sprite|SetFlipbook (Variables|Default|GetFB_Skinwalker_Walk) "/Game/Assets/PNG/AI/Skeliboi/Attack/FB_Skeliboi_Attack.FB_Skeliboi_Attack")
    (Utilities|Time|SetTimerbyFunctionName 0 "Timer_Attack_Reset" _returnvalue)
    (Utilities|Time|SetTimerbyFunctionName 0 "Do_Player_Damage" (/ _returnvalue 2.1))))

(fn TimerAttackReset
  (Variables|Default|SetIsAttacking false)
  (Sprite|SetFlipbook (Variables|Default|GetFB_Skinwalker_Walk) "/Game/Assets/PNG/AI/Skeliboi/Walk/FB_Skeliboi_walk.FB_Skeliboi_walk"))

(fn TimerDeleteSelf
  (Actor|DestroyActor))

(fn DoPlayerDamage
  (bind _can_attack (CallFunction|IsPlayerWithinRange))
  (if _can_attack
    (bind _returnvalue (Actor|GetActorOfClass "/Game/Blueprints/Player/BP_Player.BP_Player_C"))
    (if (Utilities|IsValid _returnvalue)
      (bind _dmg (CallFunction|GetDamageAmount))
      (Default|TakeDamage _returnvalue _dmg))))

(fn AnimationRotationMachine
  ;[1 1 1] If player is moving to the right, set flipbook rotation
  (if (> (.X (Math|Vector|BreakVector (Transformation|GetVelocity))) 0.0)
    (Transformation|SetRelativeRotation (Variables|Default|GetFB_Skinwalker_Walk) "0,180.000000, 0" false false)
    (else
      ;[1 1 1] Check if player is moving to the left, set flipbook rotation
      (if (< (.X (Math|Vector|BreakVector (Transformation|GetVelocity))) 0.0)
        (Transformation|SetRelativeRotation (Variables|Default|GetFB_Skinwalker_Walk) "0, 0, 0" false false)))))

(fn GetDamageAmount
  (bind _asbp_game_instance (Utilities|Casting|CastToBP_GameInstance (Game|GetGameInstance)))
  (bind _difficulty (Default|GetDifficulty _asbp_game_instance))
  (switch int _difficulty
    (:0
      ;[1 1 1] Easy
      (return 5))
    (:1
      ;[1 1 1] Normal
      (return 10))
    (:2
      ;[1 1 1] Hard
      (return 15))
    (:3
      ;[1 1 1] Inhuman
      (return 30))))